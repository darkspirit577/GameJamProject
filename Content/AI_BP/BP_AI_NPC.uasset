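; AI controller for BP_NPC pawns that drives patrol and player-sighting state through a behavior tree.
; On BeginPlay it runs BT_NPC, caches the controlled pawn and copies the loop and wait settings from that pawn's PatrolPath into the Blackboard.
; AI Perception updates write the stimulus's sensed result to CanSeePlayer, without checking which actor was sensed.
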(event `self.ReceiveBeginPlay`
  (`self.RunBehaviorTree` "/Game/AI_BP/BT_NPC.BT_NPC")
  (bind _asbp_npc (cast `/Game/AI_BP/BP_NPC` (`self.K2_GetPawn`)))
  (bind _output_get (set `self.MyPawn` _asbp_npc))
  (`BlackboardComponent.SetValueAsBool` (`AIBlueprintHelperLibrary.GetBlackboard` null) "LoopRoute" (`/Game/AI_BP/BP_PatrolRoute.IsLooping` (`/Game/AI_BP/BP_NPC.PatrolPath` _output_get)))
  (`BlackboardComponent.SetValueAsFloat` (`AIBlueprintHelperLibrary.GetBlackboard` null) "WaitTime" (`/Game/AI_BP/BP_PatrolRoute.WaitValue` (`/Game/AI_BP/BP_NPC.PatrolPath` (`self.MyPawn`)))))

(event `self.AIPerception.OnTargetPerceptionUpdated`
  (params (Actor :type "Actor Object Reference") (Stimulus :type "AIStimulus Structure"))
  (`BlackboardComponent.SetValueAsBool` (`AIBlueprintHelperLibrary.GetBlackboard` null) "CanSeePlayer" (`.bSuccessfullySensed` (break `AIStimulus` Stimulus))))

(fn `UserConstructionScript`)