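; BP_Spawner is an actor that populates its box volume with BP_NPC pawns running BT_NPC when play begins.
; For each spawn it line-traces downward against WorldStatic from high above random points in the box, with debug drawing on.
; The impact point, passed through a random-yaw transform built at that same point, becomes the spawn location, without a hit check.
; Each spawned pawn then gets its default controller.
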(event `self.ReceiveBeginPlay`
  (bind (_origin _boxextent) (`KismetSystemLibrary.GetComponentBounds` (`self.Box`)))
  (bind _returnvalue (`KismetMathLibrary.MakeVector` (.x (`KismetMathLibrary.RandomPointInBoundingBox` _origin _boxextent)) (.y (`KismetMathLibrary.RandomPointInBoundingBox` _origin _boxextent)) (+ (.z (`KismetMathLibrary.RandomPointInBoundingBox` _origin _boxextent)) 10000.0)))
  (for _ (range (+ (`self.SpawnAmount`) 1))
    (bind _outhit (`KismetSystemLibrary.LineTraceSingleForObjects` :`Start` _returnvalue :`End` (+ _returnvalue (* (* (`self.GetActorUpVector`) -1) 15000.0)) :`ObjectTypes` (`|MakeArray` "ObjectTypeQuery1" :!type "EObjectTypeQuery Enum") :`DrawDebugType` "ForDuration"))
    (bind (_bblockinghit _binitialoverlap _time _distance _location _impactpoint) (`GameplayStatics.BreakHitResult` _outhit))
    (bind _returnvalue_2 (`AIBlueprintHelperLibrary.SpawnAIFromClass` "/Game/AI_BP/BP_NPC.BP_NPC_C" "/Game/AI_BP/BT_NPC.BT_NPC" (`KismetMathLibrary.TransformLocation` (`KismetMathLibrary.MakeTransform` _impactpoint (`KismetMathLibrary.MakeRotator` 0.0 0.0 (`KismetMathLibrary.RandomFloat`))) _impactpoint)))
    (`Pawn.SpawnDefaultController` _returnvalue_2)))

(fn `UserConstructionScript`)