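; BP_EdgeBoi is a player-controlled character with cursor aiming and a shotgun attack.
; Movement input uses a zero-yaw rotator built from control pitch, so it ignores camera yaw, while Tick moves AimCursor to the point under the mouse.
; Holding right mouse runs a timeline whose event track calls ShotShogun.
; Each shot spawns eleven projectiles at the gun's barrel socket, with velocities randomized in a cone around the flattened capsule-to-cursor direction.
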(event `InputAxis|MoveForward`
  (params (AxisValue :type "Float (single-precision)"))
  ;[1 1 1] Movement
  (`self.AddMovementInput` (* (`KismetMathLibrary.GetForwardVector` (`KismetMathLibrary.MakeRotator` 0.0 (.pitch (`self.GetControlRotation`)))) AxisValue)))

(event `InputAxis|MoveRight`
  (params (AxisValue :type "Float (single-precision)"))
  ;[1 1 1] Movement
  (`self.AddMovementInput` (* (`KismetMathLibrary.GetRightVector` (`KismetMathLibrary.MakeRotator` 0.0 (.pitch (`self.GetControlRotation`)))) AxisValue)))

(event `self.ReceiveTick`
  (params (DeltaSeconds :type "Float (single-precision)"))
  (bind (_bblockinghit _binitialoverlap _time _distance _location _impactpoint) (`GameplayStatics.BreakHitResult` (`PlayerController.GetHitResultUnderCursorByChannel` (`GameplayStatics.GetPlayerController` 0) "TraceTypeQuery1" false)))
  (`SceneComponent.K2_SetWorldLocation` (`self.AimCursor`) _impactpoint false false)
  (set `self.CursorLocation` _impactpoint))

(event `Key|RightMouseButton`
  (params (Key :type "Key Structure"))
  (:`Pressed`
    (`Timeline|Timeline_0` :!via `PlayFromStart` :!label _label
      (:`NewTrack_0`
        (`self.ShotShogun`))))
  (:`Released`
    (goto _label :!via `Stop`)))

(fn `ShotShogun`
  (bind (_returnvalue_x _returnvalue_y) (`KismetMathLibrary.BreakVector` (`SceneComponent.K2_GetComponentLocation` (`self.CapsuleComponent`))))
  (`|ExecutionSequence`
    (:`then_0`
      _)
    (:`then_1`
      _)
    (:`then_2`
      _)
    (:`then_3`
      _)
    (:`then_4`
      _)
    (:`then_5`
      _)
    (:`then_6`
      _)
    (:`then_7`
      _)
    (:`then_8`
      _)
    (:`then_9`
      _)
    (:`then_10`
      _))
  (`|SpawnActorFromClass` "/Game/Perso/projectile.Projectile_C" (`KismetMathLibrary.MakeTransform` (`SceneComponent.GetSocketLocation` (`self.Gune`) "EndBarrel")) "Undefined" "OverrideRootScale" null (* (`KismetMathLibrary.RandomUnitVectorInConeInDegrees` (- (`KismetMathLibrary.MakeVector` (.x (`self.CursorLocation`)) (.y (`self.CursorLocation`))) (`KismetMathLibrary.MakeVector` _returnvalue_x _returnvalue_y)) 15.0) 4000.0) 1.0 null))

(fn `UserConstructionScript`)